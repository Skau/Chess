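; Chess game mode Blueprint that shows the winner screen when the game ends.
; Tick polls GetIfGameIsOver, then uses GetWhiteWon to pick the WhiteWon or BlackWon widget and add it to the first player's viewport.
; A three-second Delay precedes RemoveFromParent.
; No once-only guard exists, so widget creation repeats every tick while the game-over check stays true.
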(event `self.ReceiveBeginPlay`)

(event `self.ReceiveTick`
  (params (DeltaSeconds :type "Float (single-precision)"))
  (if (`self.GetIfGameIsOver`)
    (if (`self.GetWhiteWon`)
      (bind _returnvalue (`|CreateWidget` "/Game/UI/WhiteWon.WhiteWon_C" (`GameplayStatics.GetPlayerController` 0)))
      (`UserWidget.AddToViewport` _returnvalue 0)
      (`KismetSystemLibrary.Delay` 3.0)
      (`Widget.RemoveFromParent` _returnvalue)
      (else
        (bind _returnvalue_2 (`|CreateWidget` "/Game/UI/BlackWon.BlackWon_C" (`GameplayStatics.GetPlayerController` 0)))
        (`UserWidget.AddToViewport` _returnvalue_2 0)
        (`KismetSystemLibrary.Delay` 3.0)
        (`Widget.RemoveFromParent` _returnvalue_2)))))

(fn `UserConstructionScript`)