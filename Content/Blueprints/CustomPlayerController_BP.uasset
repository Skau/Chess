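; Player controller Blueprint for a chess game that manages the menu and in-game HUD widgets.
; BeginPlay creates the menu, mini menu, selected-piece and turn widgets, hiding all but the menu.
; Tick caches the clicked piece and polls the game mode to toggle HUD visibility and the menu-open flag.
; On game over, Tick creates a win widget every frame, using the WhiteWon class for both winners; stats and hover widget nodes are unconnected.
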(event `self.ReceiveBeginPlay`
  (`|ExecutionSequence`
    (:`then_0`
      (bind _returnvalue (`|CreateWidget` "/Game/UI/Menu.Menu_C"))
      (bind _output_get (set `self.MenuWidget` _returnvalue))
      (`UserWidget.AddToViewport` _output_get 0))
    (:`then_1`
      (bind _returnvalue_2 (`|CreateWidget` "/Game/UI/MiniMenu.MiniMenu_C"))
      (bind _output_get_2 (set `self.MiniMenu` _returnvalue_2))
      (`UserWidget.AddToViewport` _output_get_2 0)
      (`Widget.SetVisibility` _output_get_2 "Hidden"))
    (:`then_2`
      (bind _returnvalue_3 (`|CreateWidget` "/Game/UI/CurrentPieceClickedText.CurrentPieceClickedText_C"))
      (bind _output_get_3 (set `self.SelectedPieceWidget` _returnvalue_3))
      (`UserWidget.AddToViewport` _output_get_3 0)
      (`Widget.SetVisibility` _output_get_3 "Hidden"))
    (:`then_3`
      (bind _returnvalue_4 (`|CreateWidget` "/Game/UI/CurrentTurnText.CurrentTurnText_C"))
      (bind _output_get_4 (set `self.CurrentTurnWidget` _returnvalue_4))
      (`UserWidget.AddToViewport` _output_get_4 0)
      (`Widget.SetVisibility` _output_get_4 "Hidden"))))

(event `self.ReceiveTick`
  (params (DeltaSeconds :type "Float (single-precision)"))
  (bind _minimenu (`self.MiniMenu`))
  (bind _currentturnwidget (`self.CurrentTurnWidget`))
  (bind _selectedpiecewidget (`self.SelectedPieceWidget`))
  (bind _aschess_game_mode_base_bp (cast `/Game/Blueprints/ChessGameModeBase_BP` (`GameplayStatics.GetGameMode`) :!pure true))
  (`|ExecutionSequence`
    (:`then_0`
      (if (`ChessGameModeBase.GetIfGameIsOver` _aschess_game_mode_base_bp)
        (if (`ChessGameModeBase.GetWhiteWon` _aschess_game_mode_base_bp)
          (bind _returnvalue (`|CreateWidget` "/Game/UI/WhiteWon.WhiteWon_C"))
          (bind _output_get (set `self.WhiteWonWidget` _returnvalue))
          (`UserWidget.AddToViewport` _output_get 0)
          (else
            (bind _returnvalue_2 (`|CreateWidget` "/Game/UI/WhiteWon.WhiteWon_C"))
            (bind _output_get_2 (set `self.BlackWonWidget` _returnvalue_2))
            (`UserWidget.AddToViewport` _output_get_2 0)))))
    (:`then_1`
      (set `self.SelectedChessPiece` (`self.GetCurrentChessPieceClicked`)))
    (:`then_2`
      (if (`ChessGameModeBase.GetGameIsActive` (cast `/Game/Blueprints/ChessGameModeBase_BP` (`GameplayStatics.GetGameMode`) :!pure true))
        (`self.SetMenuWindowOpenBool` false)
        (if (xor (`KismetSystemLibrary.IsValid` (`self.BlackWonWidget`)) (`KismetSystemLibrary.IsValid` (`self.WhiteWonWidget`)))
          (`Widget.SetVisibility` _currentturnwidget "Hidden" :!label _label)
          (`Widget.SetVisibility` _selectedpiecewidget "Hidden")
          (`Widget.SetVisibility` _minimenu "Hidden")
          (else
            (`Widget.SetVisibility` _currentturnwidget "Visible")
            (`Widget.SetVisibility` _selectedpiecewidget "Visible")
            (`Widget.SetVisibility` _minimenu "Visible")))
        (else
          (`self.SetMenuWindowOpenBool` true)
          (goto _label))))))

(fn `UserConstructionScript`)